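; Berry bush actor that covers itself with berry pickups when play begins.
; BeginPlay sizes the Berries array to BerryAmount, then spawns a scaled-down BP_BerryPickup for each slot, disables its physics and stores it.
; Each position takes an evenly stepped X and random Y and Z within the BerrySpawnSphere radius, normalized to project the berry onto the sphere's surface.
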(event EventBeginPlay
  (bind _berryspawnsphere (Variables|Default|GetBerrySpawnSphere))
  (bind _berryspawnsphere_2 (Variables|Default|GetBerrySpawnSphere))
  (bind _berries (Variables|Default|GetBerries))
  (bind _returnvalue (Components|Sphere|GetScaledSphereRadius _berryspawnsphere))
  (bind _returnvalue_2 (Components|Sphere|GetScaledSphereRadius _berryspawnsphere_2))
  ;[0.2187 0.9901 1] Sets Array Size based off amount of berries set and then Loops for each slot
  (Utilities|Array|Resize _berries (Variables|Default|GetBerry%20Amount))
  (Variables|Default|SetIncrement (/ (* (Components|Sphere|GetScaledSphereRadius (Variables|Default|GetBerrySpawnSphere)) 2.0) (Math|Conversions|ToFloat(Integer) (Variables|Default|GetBerry%20Amount))))
  (for (_ _array_index) _berries
    ;[1 0.2435 0.8955] Spawns berry, removes its physics and places it into array
    (bind _returnvalue_3 (Game|SpawnActorfromClass "/Game/GameContent/Blueprints/PickupItems/BP_BerryPickup.BP_BerryPickup_C" (Math|Transform|MakeTransform (+ (Transformation|GetWorldLocation (Variables|Default|GetBerrySpawnSphere)) (* (Components|Sphere|GetScaledSphereRadius (Variables|Default|GetBerrySpawnSphere)) (Math|Vector|Normalize (Math|Vector|MakeVector (+ (* _array_index (Variables|Default|GetIncrement)) (* (Components|Sphere|GetScaledSphereRadius (Variables|Default|GetBerrySpawnSphere)) -1.0)) (Math|Random|RandomFloatinRange (* _returnvalue_2 -1.0) _returnvalue_2) (Math|Random|RandomFloatinRange (* _returnvalue -1.0) _returnvalue))))) "0, 0, 0" "0.200000,0.200000,0.200000") "AlwaysSpawn" "MultiplyWithRoot" 0 0))
    (Physics|SetSimulatePhysics (Variables|/Script/CollabGroup06Project.BerryPickup|Get_CollisionComponent _returnvalue_3) false)
    (Utilities|Array|SetArrayElem _berries _array_index _returnvalue_3)))

(fn ConstructionScript)