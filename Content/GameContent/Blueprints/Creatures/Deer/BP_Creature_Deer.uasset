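; Deer creature Blueprint, a child class that supplies the deer's responses to animal action and feed events.
; The bespoke action prints a deer greeting and plays the MSSDeer sound.
; Feed marks the deer photographable, prints a debug string and plays the MSSDeerFeed sound, with no berry check in this graph despite its comment.
; Interact is empty and construction only calls the parent.
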(event EventBeginPlay
  (|CallParentFunction) ; This node is disabled and will not be called.\nDrag off pins to build functionality.
)

(event Collision|EventActorBeginOverlap
  (params (OtherActor :type Actor%20Object%20Reference)))

(event EventTick
  (params (DeltaSeconds :type Float%20%28single-precision%29)))

(event EventFeed
  ;[1 1 1] Alternative Interaction that peforms check if player has a berry and animal can be fed
  (Variables|Default|Set_IsPhotographable true)
  (Development|PrintString "Bosh")
  (Audio|Components|Audio|Play (Variables|Default|GetMSS_DeerFeed) 0.0))

(event EventBespokeAnimalAction
  (Development|PrintString "Mi! I am a deer!" true true "(R=1.000000,G=0.916554,B=0.497187,A=1.000000)")
  (Audio|Components|Audio|Play (Variables|Default|GetMSS_Deer) 0.0))

(event EventInteract
  ;[1 1 1] DOES NOTHING
)

(fn ConstructionScript
  (|CallParentFunction))