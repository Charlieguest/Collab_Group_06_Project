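; Berry Bird creature that hides in a bush as a berry until a one-time interaction reveals it as a photographable kiwi.
; Interacting swaps meshes, teleports it out, plays a startled sound and launches it with temporary capsule physics before resetting it upright and showing hearts.
; A self-rearming random timer then drives navmesh hops, with chirp and footstep sounds capped by a counter.
; BeginPlay prepares a hidden thought bubble with a puzzle-aid image.
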(event Custom|HOP
  (bind _self self)
  ;[0.3638 1 0.9701] Hop
  (Components|Animation|PlayAnimation (Variables|Character|GetMesh) "/Game/Art/CharacterModels/KiwiModel/Animations/Kiwi_Hop.Kiwi_Hop" true)
  (CallFunction|PlayChirp)
  (bind _randomlocation (Class|NavigationSystemV1|GetRandomLocationinNavigableRadius (Transformation|GetActorLocation _self) (Variables|Default|GetHopRadius) 0 0))
  (AI|AIMoveTo _self _randomlocation 0 5.0 false
    (:then
      (Utilities|FlowControl|Delay (Variables|Default|GetHop%20Animation%20Duration))
      (Variables|Default|SetTime%20before%20Hop (Math|Random|RandomFloatinRange (Variables|Default|GetHopMinTime) (Variables|Default|GetHopMaxTime)))
      (Components|Animation|PlayAnimation (Variables|Character|GetMesh) "/Game/Art/CharacterModels/KiwiModel/Animations/Kiwi_Idle1.Kiwi_Idle1" true)
      ;[0.9257 0.4022 1] Resets Velocity and rotation to stand upright
      (Utilities|Time|SetTimerbyEvent (delegate Custom|HOP) (Variables|Default|GetTime%20before%20Hop))
      (Rendering|SetVisibility (Variables|Default|GetHeartsVFX) true false))))

(event Custom|PlayChirp
  (if (not (>= (Variables|Default|GetChirpCounter) (Variables|Default|GetChirpThreshold)))
    (Audio|Components|Audio|Play (Variables|Default|GetMSS_BirdSqueak) 0.0)
    (Audio|Components|Audio|Play (Variables|Default|GetMSS_CreatureFootstep) 0.0)
    (Math|Integer|IncrementInt (Variables|Default|GetChirpCounter))))

(event EventBeginPlay
  (bind _widgetthoughtbubble (Variables|Default|GetWidgetThoughtBubble))
  (bind _returnvalue (UserInterface|GetUserWidgetObject _widgetthoughtbubble))
  (bind _asc_ui_thought_bubble (Utilities|Casting|CastToC_UI_ThoughtBubble _returnvalue))
  (Variables|Default|SetThoughtBubbleInstance _asc_ui_thought_bubble)
  (Default|SetDesiredImage _asc_ui_thought_bubble (Variables|Default|GetPuzzleAidTexture))
  (Widget|SetVisibility _returnvalue "Hidden"))

(event EventInteract
  (bind _capsulecomponent (Variables|Default|GetCapsuleComponent))
  (bind _capsulecomponent_2 (Variables|Default|GetCapsuleComponent))
  (Utilities|FlowControl|DoOnce false
    (:Completed
      ;[0.2885 0.7877 1] Hides berry asset, Sets Kiwi Asset, Changes size of kiwi
      (Development|SetHiddeninGame (Variables|Default|GetTempmesh%20-%20Berry) true false)
      (Components|SkeletalMesh|SetSkeletalMeshAsset (Variables|Character|GetMesh) "/Game/Art/CharacterModels/KiwiModel/Kiwi_Mesh.Kiwi_Mesh")
      (Transformation|SetRelativeScale3D (Variables|Default|GetCapsuleComponent) "1.000000,1.000000,1.000000")
      ;[1 0.2292 0.2292] Moves bird out of bush via teleport
      (Transformation|SetActorLocation (+ (Transformation|GetActorLocation) (Variables|Default|Getteleport%20offset)) false true)
      ;[0.6013 1 0.6231] Enable Collisions and physics
      (Collision|SetCollisionEnabled _capsulecomponent_2 "QueryAndPhysics")
      (Collision|SetCollisionResponsetoAllChannels _capsulecomponent_2 "ECR_Block")
      (Collision|SetCollisionResponsetoChannel _capsulecomponent_2 "ECC_GameTraceChannel1" "ECR_Ignore")
      (Collision|SetCollisionResponsetoChannel _capsulecomponent_2 "ECC_Visibility" "ECR_Ignore")
      (Physics|SetSimulatePhysics _capsulecomponent_2 true)
      (Physics|SetEnableGravity _capsulecomponent_2 true)
      (Variables|/Script/Engine.CharacterMovementComponent|SetGravityScale (Variables|Character|GetCharacterMovement) 1.0)
      ;[1 1 1] Startled sound plays
      (Audio|Components|Audio|Play (Variables|Default|GetMSS_BirdStartled) 0.0)
      ;[1 0.8954 0.4689] Launch the bird out the bush
      (Physics|AddImpulse (Variables|Default|GetCapsuleComponent) (Variables|Default|GetLaunch) "None" true)
      ;[0.5282 1 0.4428] Delay before Reseting velocity
      (Utilities|FlowControl|Delay (Variables|Default|GetDelay%20before%20Standing%20up))
      ;[0.9257 0.4022 1] Resets Velocity and rotation to stand upright
      (Physics|SetSimulatePhysics _capsulecomponent false)
      (Physics|SetPhysicsLinearVelocity _capsulecomponent "0, 0, 0" false "None")
      (Class|PrimitiveComponent|SetPhysicsAngularVelocityinDegrees _capsulecomponent "0, 0, 0" false "None")
      (Transformation|SetActorRotation (Math|Rotator|MakeRotator 0.0 0.0 (.yaw (Transformation|GetActorRotation))))
      (Variables|Default|Set_IsPhotographable true)
      (Variables|Default|SetTime%20before%20Hop (Math|Random|RandomFloatinRange (Variables|Default|GetHopMinTime) (Variables|Default|GetHopMaxTime)))
      (Utilities|Time|SetTimerbyEvent (delegate Custom|HOP) (Variables|Default|GetTime%20before%20Hop))
      (Rendering|SetVisibility (Variables|Default|GetHeartsVFX) true false))))

(fn ConstructionScript
  (|CallParentFunction))