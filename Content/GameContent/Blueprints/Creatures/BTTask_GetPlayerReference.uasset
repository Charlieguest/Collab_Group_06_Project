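; Behavior tree task for creature AI that stores a reference to the player character in the Player blackboard key.
; It succeeds at once if the key already holds a valid actor.
; Otherwise it searches for all BP_PlayerCharacter actors, writes the first one to the key and succeeds, or fails if none exists.
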(event EventReceiveExecuteAI
  (params (OwnerController :type AI%20Controller%20Object%20Reference) (ControlledPawn :type Pawn%20Object%20Reference))
  ;[0.2604 0.2604 0.2604] Asigns player
  (Utilities|IsValid (AI|BehaviorTree|GetBlackboardValueasActor (Variables|Default|GetPlayer))
    (:Is%20Valid
      (AI|BehaviorTree|FinishExecute true))
    (:Is%20Not%20Valid
      (bind _outactors (Actor|GetAllActorsOfClass "/Game/GameContent/Blueprints/Player/BP_PlayerCharacter.BP_PlayerCharacter_C"))
      (if (Utilities|Array|IsValidIndex _outactors)
        (Class|BTFunctionLibrary|SetBlackboardValueasObject (Variables|Default|GetPlayer) (Utilities|Array|Get(acopy) _outactors))
        (AI|BehaviorTree|FinishExecute true)
        (else
          (AI|BehaviorTree|FinishExecute false))))))