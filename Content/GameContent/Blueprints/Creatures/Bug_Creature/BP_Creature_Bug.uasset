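; Bug creature that, once interacted with, walks a chain of waypoints and then heads to its nest.
; A looping timer drives AI moves toward the current waypoint, and waypoints call WaypointHit to advance the index.
; After the nest move, a positive wait time makes it photographable, then teleports it to its start after the delay.
; That reset also re-arms the DoOnce gating Interact, so the run can repeat.
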(event Custom|Move%20to%20waypoint
  ;[0.4091 1 0.5146] Checks if waypoint is hit - if it is it increments, checks if its time for nest, and carries on
  (if (Variables|Default|GetCurrent%20Waypoint%20Hit)
    (Development|PrintString "KZZT - TIS ARRIVED!! (1)")
    (bind _result (Math|Integer|IncrementInt (Variables|Default|GetCurrentIndex))
      (:%20%20
        (Variables|Default|SetCurrent%20Waypoint%20Hit false)
        (if (<= (Utilities|Array|Length (Variables|Default|GetWaypoints)) _result)
          (CallFunction|MovetoNest))))
    (else
      (AI|AIMoveTo self "0, 0, 0" (Utilities|Array|Get(acopy) (Variables|Default|GetWaypoints) (Variables|Default|GetCurrentIndex)) (Variables|Default|GetAcceptance%20Radius) false
        (:OnSuccess
          (Development|PrintString "KZZT - TIS ARRIVED!! (2)"))
        (:OnFail
          (Development|PrintString "KZZT - ON ME WAY"))))))

(event Custom|Move%20to%20Nest
  (bind _time_to_wait_before_reseting (Variables|Default|GetTime%20to%20wait%20before%20reseting))
  ;[0.2663 0.3722 1] When Nest time arrives, it stops the movement timer and moves to the nest
  (Development|PrintString "KZZT - HUZZAH HOME SWEET HOME")
  (Utilities|Time|ClearandInvalidateTimerbyHandle (Variables|Default|GetMove))
  (AI|AIMoveTo self "0, 0, 0" (Variables|Default|GetNest) 5.0 false
    (:then
      (if (> _time_to_wait_before_reseting 0.0)
        (Variables|Default|Set_IsPhotographable true)
        (Utilities|FlowControl|Delay _time_to_wait_before_reseting)
        (Variables|Default|Set_IsPhotographable true)
        (Development|PrintString "KZZT - My existence is to be doomed in this loop forever" true true "(R=0.255208,G=0.000000,B=0.017134,A=1.000000)")
        (CallFunction|FullReset)))))

(event Custom|Reset%20DO%20Once
  ;[1 0.4115 0.4115] Replace with Interact - Initial Start
  (Utilities|FlowControl|DoOnce false) ; enters at Reset
)

(event Custom|Full%20Reset
  (bind _starting_transform (Variables|Default|GetStarting%20Transform))
  ;[1 0.237 0.7317] Resets the do once and moves bug to start
  (Utilities|Time|ClearandInvalidateTimerbyHandle (Variables|Default|GetMove))
  (Variables|Default|SetCurrent%20Waypoint%20Hit false)
  (Transformation|Teleport (.location _starting_transform) (.rotation _starting_transform))
  (CallFunction|ResetDOOnce))

(event Custom|Waypoint%20Hit
  ;[0.3045 0.3177 0.2976] Called By Waypoints
  (Variables|Default|SetCurrent%20Waypoint%20Hit true))

(event EventBeginPlay
  (Variables|Default|SetStarting%20Transform (Transformation|GetActorTransform))
  (|CallParentFunction))

(event EventInteract
  ;[1 0.4115 0.4115] Replace with Interact - Initial Start
  (Development|PrintString "KZZT - Bug Touched")
  (Utilities|FlowControl|DoOnce false
    (:Completed
      (Variables|Default|SetCurrentIndex 0)
      (bind _returnvalue (Utilities|Time|SetTimerbyEvent (delegate Custom|Move%20to%20waypoint) (Variables|Default|GetTime%20Between%20move%20checks) true))
      (Variables|Default|SetMove _returnvalue))))

(fn ConstructionScript
  (|CallParentFunction))