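; Behavior Tree task that makes an AI creature walk up to the blackboard Player when that player is standing still.
; On execute it fails if player speed exceeds a tolerance, otherwise it sets a timer for the required standstill time.
; The timer event moves the pawn within an acceptance radius of the player's location and reports the result.
; The movement re-check meant to cancel the approach during the wait is only called from disconnected nodes.
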(event Custom|ApproachPlayer
  ;[0.6662 0.3124 1] If Approach is still true approach the player
  (Variables|Default|SetLoopingCheck false)
  (if (Variables|Default|GetApproach?)
    (AI|AIMoveTo (stale EventReceiveExecuteAI ControlledPawn) (Transformation|GetActorLocation (AI|BehaviorTree|GetBlackboardValueasActor (Variables|Default|GetPlayer))) 0 (Variables|Default|GetRadius%20from%20player%20to%20move%20to) true
      (:OnSuccess
        (Variables|Default|SetFinished true)
        (AI|BehaviorTree|FinishExecute true))
      (:OnFail
        (Variables|Default|SetFinished true :!label _label)
        (AI|BehaviorTree|FinishExecute false)))
    (else
      (goto _label))))

(event Custom|Check%20if%20player%20moved
  ;[0.375 1 1] Checks if player moved
  (if (Variables|Default|GetFinished)
    (Variables|Default|SetLoopingCheck false)
    (elif (> (Math|Vector|VectorLength (Transformation|GetVelocity (AI|BehaviorTree|GetBlackboardValueasActor (Variables|Default|GetPlayer)))) (Variables|Default|GetErrorTolerence%20for%20standing%20still))
      (Variables|Default|SetApproach? false)
      (Variables|Default|SetLoopingCheck false))))

(event EventReceiveExecuteAI
  (params (OwnerController :type AI%20Controller%20Object%20Reference) (ControlledPawn :type Pawn%20Object%20Reference))
  ;[1 0.5521 0.5521] If Player isn't moving, starts a timer to approach
  (if (not (> (Math|Vector|VectorLength (Transformation|GetVelocity (AI|BehaviorTree|GetBlackboardValueasActor (Variables|Default|GetPlayer)))) (Variables|Default|GetErrorTolerence%20for%20standing%20still)))
    (Variables|Default|SetApproach? true)
    (Variables|Default|SetLoopingCheck true)
    (Utilities|Time|SetTimerbyEvent (delegate Custom|ApproachPlayer) (Variables|Default|GetTimeRequiredStandingStill))
    (else
      (Variables|Default|SetFinished true)
      (AI|BehaviorTree|FinishExecute false))))