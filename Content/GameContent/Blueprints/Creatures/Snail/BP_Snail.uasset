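; BP_Snail is a snail creature that can be scanned and becomes photographable when given an item.
; OnScanned prints a debug hint asking for a rock and calls ShowBubble.
; An ItemDevTest overlapping PlayerInteractionZone sets IsPhotographable and prints a happy message.
; The player lookup and yaw-only look-at rotation toward a nearby target are disconnected, as BeginPlay and Tick are empty.
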(event OnComponentBeginOverlap(PlayerInteractionZone)
  (params (OverlappedComponent :type Primitive%20Component%20Object%20Reference) (OtherActor :type Actor%20Object%20Reference) (OtherComp :type Primitive%20Component%20Object%20Reference) (OtherBodyIndex :type Integer) (bFromSweep :type Boolean) (SweepResult :type Hit%20Result%20Structure%20%28by%20ref%29))
  ;[0.2473 1 0] On Overlap
  (Utilities|Casting|CastToItemDevTest OtherActor)
  (if true
    (Variables|Default|Set_IsPhotographable true)
    (Development|PrintString "Hello, Im Happy")))

(event EventBeginPlay
  ;[0 0 0] Rotate towards player
)

(event Collision|EventActorBeginOverlap
  (params (OtherActor :type Actor%20Object%20Reference)))

(event EventTick
  (params (DeltaSeconds :type Float%20%28single-precision%29))
  ;[0 0 0] Rotate towards player
)

(event EventOnScanned
  ;[1 0.9952 0] Debug stuff
  (Development|PrintString "Im in my shell, if you want to see me give me rock")
  (CallFunction|ShowBubble))

(fn ConstructionScript
  (|CallParentFunction))