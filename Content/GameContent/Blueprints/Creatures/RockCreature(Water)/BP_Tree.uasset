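; BP_Tree is an interactable tree that awakens the rock creature frog.
; On BeginPlay it finds and stores the BP_RockCreature, assuming only one exists, while a box overlap tracks whether the player is in range.
; An in-range interaction fires once, activating leaf and water particles and running a timeline that fades the creature's material Blend parameter, then calls ActivateFrog.
; An unconnected snippet would make the frog photographable.
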(event OnComponentBeginOverlap(Box)
  (params (OverlappedComponent :type Primitive%20Component%20Object%20Reference) (OtherActor :type Actor%20Object%20Reference) (OtherComp :type Primitive%20Component%20Object%20Reference) (OtherBodyIndex :type Integer) (bFromSweep :type Boolean) (SweepResult :type Hit%20Result%20Structure%20%28by%20ref%29))
  (if (Utilities|ClassIsChildOf (Utilities|GetClass OtherActor) "/Game/GameContent/Blueprints/Player/BP_PlayerCharacter.BP_PlayerCharacter_C")
    (Variables|Default|SetplayerOverlapping true)
    (Development|PrintString "overlap")))

(event OnComponentEndOverlap(Box)
  (params (OverlappedComponent :type Primitive%20Component%20Object%20Reference) (OtherActor :type Actor%20Object%20Reference) (OtherComp :type Primitive%20Component%20Object%20Reference) (OtherBodyIndex :type Integer))
  (if (Utilities|ClassIsChildOf (Utilities|GetClass OtherActor) "/Game/GameContent/Blueprints/Player/BP_PlayerCharacter.BP_PlayerCharacter_C")
    (Variables|Default|SetplayerOverlapping false)))

(event EventInteract
  (if (Variables|Default|GetplayerOverlapping)
    (Utilities|FlowControl|DoOnce false
      (:Completed
        (Components|Activation|Activate (Variables|Default|GetLeafParticle) false)
        (Components|Activation|Activate (Variables|Default|Getns_Water) false)
        (Development|PrintString "activated")
        ;[1 1 1] fade the frog material from inactive to active
        (bind _newtrack_0 (Timeline|Timeline Play)
          (:Update
            (Rendering|Material|SetScalarParameterValue (Variables|/Game/GameContent/Blueprints/Creatures/RockCreature(Water)/BP_RockCreature.BP_RockCreature_C|GetBlendMaterial (Variables|Default|GetRockCreature)) "Blend" _newtrack_0 :!class /Script/Engine.MaterialInstanceDynamic))
          (:Finished
            (Default|ActivateFrog (Variables|Default|GetRockCreature))))))))

(event EventBeginPlay
  ;[1 1 1] since there will only ever be one frog this should work fine
  (bind _outactors (Actor|GetAllActorsOfClass "/Game/GameContent/Blueprints/Creatures/RockCreature(Water)/BP_RockCreature.BP_RockCreature_C"))
  (for _array_element _outactors
    (Variables|Default|SetRockCreature _array_element)))

(fn ConstructionScript)