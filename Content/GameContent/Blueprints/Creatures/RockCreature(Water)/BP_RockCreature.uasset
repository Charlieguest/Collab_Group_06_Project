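; Water rock creature that becomes photographable once the player interacts with it up close.
; A box overlap tracks whether BP_PlayerCharacter is in range, and Interact only takes effect while it is.
; A DoOnce gate makes the first valid interaction activate the leaf and water particles and set IsPhotographable, with debug prints along the way.
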(event OnComponentBeginOverlap(Box)
  (params (OverlappedComponent :type Primitive%20Component%20Object%20Reference) (OtherActor :type Actor%20Object%20Reference) (OtherComp :type Primitive%20Component%20Object%20Reference) (OtherBodyIndex :type Integer) (bFromSweep :type Boolean) (SweepResult :type Hit%20Result%20Structure%20%28by%20ref%29))
  (if (Utilities|ClassIsChildOf (Utilities|GetClass OtherActor) "/Game/GameContent/Blueprints/Player/BP_PlayerCharacter.BP_PlayerCharacter_C")
    (Variables|Default|SetplayerOverlapping true)
    (Development|PrintString "overlap")))

(event OnComponentEndOverlap(Box)
  (params (OverlappedComponent :type Primitive%20Component%20Object%20Reference) (OtherActor :type Actor%20Object%20Reference) (OtherComp :type Primitive%20Component%20Object%20Reference) (OtherBodyIndex :type Integer))
  (if (Utilities|ClassIsChildOf (Utilities|GetClass OtherActor) "/Game/GameContent/Blueprints/Player/BP_PlayerCharacter.BP_PlayerCharacter_C")
    (Variables|Default|SetplayerOverlapping false)))

(event EventBeginPlay
  (|CallParentFunction) ; This node is disabled and will not be called.\nDrag off pins to build functionality.
)

(event EventInteract
  (if (Variables|Default|GetplayerOverlapping)
    (Utilities|FlowControl|DoOnce false
      (:Completed
        (Components|Activation|Activate (Variables|Default|GetLeafParticle) false)
        (Components|Activation|Activate (Variables|Default|GetWaterParticle) false)
        (Development|PrintString "activated")
        (Variables|Default|Set_IsPhotographable true)
        (Development|PrintString (Utilities|String|ToString(Boolean) (Variables|Default|Get_IsPhotographable)))))))

(fn ConstructionScript
  (|CallParentFunction))