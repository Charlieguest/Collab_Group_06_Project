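; Behavior tree task for creatures that makes the controlled pawn flee from the player when the player is moving.
; After a short delay, it compares the speed of the blackboard's Player actor against a standstill tolerance.
; If the player is moving, it runs an AI move along the direction away from them, scaled by a run distance with height offset zeroed.
; It succeeds when that move completes and fails if the move fails or the player is still.
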(event EventReceiveExecuteAI
  (params (OwnerController :type AI%20Controller%20Object%20Reference) (ControlledPawn :type Pawn%20Object%20Reference))
  (bind _returnvalue (Transformation|GetActorLocation ControlledPawn))
  (bind _distance_to_run (Variables|Default|GetDistance%20to%20run))
  (Utilities|FlowControl|Delay (Variables|Default|GetMovement%20check%20delay))
  (if (> (Math|Vector|VectorLength (Transformation|GetVelocity (AI|BehaviorTree|GetBlackboardValueasActor (Variables|Default|GetPlayer)))) (Variables|Default|GetError%20Tolerence%20For%20Standing%20Still))
    (AI|AIMoveTo ControlledPawn (+ _returnvalue (* (Math|Vector|Normalize (- _returnvalue (Transformation|GetActorLocation (AI|BehaviorTree|GetBlackboardValueasActor (Variables|Default|GetPlayer))))) (Math|Vector|MakeVector _distance_to_run _distance_to_run 0.0))) 0 5.0 false
      (:OnSuccess
        (AI|BehaviorTree|FinishExecute true))
      (:OnFail
        (AI|BehaviorTree|FinishExecute false :!label _label)))
    (else
      (goto _label))))