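; Lizard creature Blueprint whose special animal action plays a hiss, prints a debug message and fades the near-hidden lizard into view.
; The construction script assigns a dynamic material instance to the Cube, starting at minimum opacity.
; A timeline lerps that opacity up, then a timer fires UndoVis after a set duration to reverse the same timeline and fade it back out.
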(event Custom|UndoVis
  (bind _time_to_stay_visible_for (Variables|Default|GetTime%20to%20stay%20visible%20for))
  ;[1 0.8922 0.3718] Can be replaced by animation later on
  (Variables|Default|SetVisible false)
  (bind _lerpforopacity (Timeline|Becoming%20Visble ReverseFromEnd)
    (:Update
      (Rendering|Material|SetScalarParameterValue (Variables|Default|GetCubeMaterial) "Opacity" (Math|Float|Lerp (Variables|Default|GetLizard%20min%20Opacity) (Variables|Default|GetLizard%20Max%20Opacity_0) _lerpforopacity) :!class /Script/Engine.MaterialInstanceDynamic))
    (:Finished
      (if (and (Variables|Default|GetVisible) (> _time_to_stay_visible_for 0.0))
        (Utilities|Time|SetTimerbyEvent (delegate Custom|UndoVis) _time_to_stay_visible_for)))))

(event EventBeginPlay
  (|CallParentFunction))

(event EventBespokeAnimalAction
  (bind _time_to_stay_visible_for (Variables|Default|GetTime%20to%20stay%20visible%20for))
  ;[1 0.8922 0.3718] Can be replaced by animation later on
  (Development|PrintString "Zzt! I am a Lizard!" true true "(R=0.155440,G=1.000000,B=0.135417,A=1.000000)")
  (Audio|Components|Audio|Play (Variables|Default|GetMSS_LizardHiss) 0.0)
  (if (not (Variables|Default|GetVisible))
    (Variables|Default|SetVisible true)
    (bind _lerpforopacity (Timeline|Becoming%20Visble PlayFromStart)
      (:Update
        (Rendering|Material|SetScalarParameterValue (Variables|Default|GetCubeMaterial) "Opacity" (Math|Float|Lerp (Variables|Default|GetLizard%20min%20Opacity) (Variables|Default|GetLizard%20Max%20Opacity_0) _lerpforopacity) :!class /Script/Engine.MaterialInstanceDynamic))
      (:Finished
        (if (and (Variables|Default|GetVisible) (> _time_to_stay_visible_for 0.0))
          (Utilities|Time|SetTimerbyEvent (delegate Custom|UndoVis) _time_to_stay_visible_for))))))

(fn ConstructionScript
  ;[0.2317 0.4801 1] Creates a material instance of the lizard material and assigns it to the lizard
  (bind _returnvalue (Rendering|Material|CreateDynamicMaterialInstance "/Game/GameContent/Blueprints/Creatures/Lizard/Temp_LizardMaterial.Temp_LizardMaterial" "None" "None" :!class /Script/Engine.KismetMaterialLibrary))
  (bind _output_get (Variables|Default|SetCubeMaterial _returnvalue))
  (Rendering|Material|SetMaterial (Variables|Default|GetCube) 0 _output_get)
  (Rendering|Material|SetScalarParameterValue _output_get "Opacity" (Variables|Default|GetLizard%20min%20Opacity) :!class /Script/Engine.MaterialInstanceDynamic)
  (|CallParentFunction))