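; Base creature Blueprint for animals that become photographable on interaction and show a puzzle-aid thought bubble when scanned.
; A delayed scan response reveals the widget, runs a one-time BespokeAnimalAction hook (empty here), and uses timers to yaw the bubble toward the camera and later hide it.
; The bubble image flips by viewing angle.
; An overlap zone checks the player's inventory for the required item, or hides the help panel if they hold the camera.
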(event OnComponentBeginOverlap(PlayerInteractionZone)
  (params (OverlappedComponent :type Primitive%20Component%20Object%20Reference) (OtherActor :type Actor%20Object%20Reference) (OtherComp :type Primitive%20Component%20Object%20Reference) (OtherBodyIndex :type Integer) (bFromSweep :type Boolean) (SweepResult :type Hit%20Result%20Structure%20%28by%20ref%29))
  (bind _asbp_player_character (Utilities|Casting|CastToBP_PlayerCharacter OtherActor))
  (bind _output_get (Variables|Default|Set_PlayerCharacter _asbp_player_character))
  (if (Variables|/Script/CollabGroup06Project.PlayerCharacter|Get_IsHoldingCamera (Variables|Default|Get_PlayerCharacter))
    (Default|HideHelpPanel (Variables|Default|Get_PlayerCharacter))
    (else
      (Default|InventoryItemCheck (Variables|/Game/GameContent/Blueprints/Player/BP_PlayerCharacter.BP_PlayerCharacter_C|GetBP_InventoryComponent _output_get) (Variables|Default|Get_RequiredItemName) false))))

(event OnComponentEndOverlap(PlayerInteractionZone)
  (params (OverlappedComponent :type Primitive%20Component%20Object%20Reference) (OtherActor :type Actor%20Object%20Reference) (OtherComp :type Primitive%20Component%20Object%20Reference) (OtherBodyIndex :type Integer))
  (bind _asbp_player_character (Utilities|Casting|CastToBP_PlayerCharacter OtherActor))
  (Default|HideHelpPanel _asbp_player_character))

(event Custom|RotateToPlayer
  (bind _returnvalue (Game|GetPlayerCameraManager 0))
  (bind _widgetthoughtbubble (Variables|Default|GetWidgetThoughtBubble))
  (bind _returnvalue_2 (Transformation|GetWorldLocation _widgetthoughtbubble))
  (bind _transformcomponent (Variables|/Script/Engine.PlayerCameraManager|GetTransformComponent _returnvalue))
  (bind _returnvalue_3 (Transformation|GetWorldLocation _transformcomponent))
  (bind _returnvalue_4 (Math|Rotator|FindLookatRotation _returnvalue_2 _returnvalue_3))
  ;[1 1 1] Rotating Speech bubble to Player
  (Transformation|SetWorldRotation _widgetthoughtbubble (Math|Rotator|MakeRotator 0.0 0.0 (.yaw _returnvalue_4)) false false)
  (if (> (.yaw _returnvalue_4) -4e+01)
    (if (< (.yaw _returnvalue_4) 1.5e+02)
      (Default|FlipImage (Variables|Default|GetThoughtBubbleInstance) "(X=1.000000,Y=1.000000)")
      (else
        (Default|FlipImage (Variables|Default|GetThoughtBubbleInstance) "(X=-1.000000,Y=1.000000)")))
    (else
      (Default|FlipImage (Variables|Default|GetThoughtBubbleInstance) "(X=-1.000000,Y=1.000000)"))))

(event Custom|Bespoke%20Animal%20Action
  ;[1 1 1] Setting Specific Image and Then Visibility to None
)

(event Custom|ShowBubble
  ;[1 1 1] Setting Specific Image and Then Visibility to None
  (Widget|SetVisibility (UserInterface|GetUserWidgetObject (Variables|Default|GetWidgetThoughtBubble)) "Visible")
  (Utilities|Time|SetTimerbyEvent (EventDispatchers|CreateEvent :!event Custom|RotateToPlayer) 0.03 true true)
  (if (Variables|Default|Get_BeenActivated)
    _
    (else
      (Variables|Default|Set_BeenActivated true)
      (CallFunction|BespokeAnimalAction)))
  (Utilities|Time|SetTimerbyEvent (EventDispatchers|CreateEvent :!event Custom|Hide%20Bubble) 5.0))

(event Custom|Hide%20Bubble
  ;[1 1 1] Resetting visibility after 5 seconds
  (Widget|SetVisibility (UserInterface|GetUserWidgetObject (Variables|Default|GetWidgetThoughtBubble)) "Hidden"))

(event EventBeginPlay
  (bind _widgetthoughtbubble (Variables|Default|GetWidgetThoughtBubble))
  (bind _returnvalue (UserInterface|GetUserWidgetObject _widgetthoughtbubble))
  ;[1 1 1] Setting Specific Image and Then Visibility to None
  (bind _asc_ui_thought_bubble (Utilities|Casting|CastToC_UI_ThoughtBubble _returnvalue))
  (Variables|Default|SetThoughtBubbleInstance _asc_ui_thought_bubble)
  (Default|SetDesiredImage _asc_ui_thought_bubble (Variables|Default|GetPuzzleAidTexture))
  (Widget|SetVisibility _returnvalue "Hidden"))

(event EventOnScanned
  ;[1 1 1] On Scanned Interface Execution
  (Utilities|Time|SetTimerbyEvent (EventDispatchers|CreateEvent :!event Custom|ShowBubble) 2.0))

(event EventInteract
  ;[1 1 1] Set the animal to photographable
  (Variables|Default|Set_IsPhotographable true))

(fn ConstructionScript)