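; BP_CheckpointNet is a safety-net volume that teleports the player character or berry pickups overlapping its collision box to a checkpoint.
; It caches all BP_CheckpointTester actors on BeginPlay, then picks the lowest dot product of world positions as "nearest", rather than measuring distance.
; The first checkpoint only seeds that comparison without being stored as closest.
; Before teleporting, it toggles physics simulation on a primitive component to stop movement.
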(event OnComponentBeginOverlap(SafetyCollisionBox)
  (params (OverlappedComponent :type Primitive%20Component%20Object%20Reference) (OtherActor :type Actor%20Object%20Reference) (OtherComp :type Primitive%20Component%20Object%20Reference) (OtherBodyIndex :type Integer) (bFromSweep :type Boolean) (SweepResult :type Hit%20Result%20Structure%20%28by%20ref%29))
  ;[1 1 1] Detect Player entering net
  (bind _asbp_player_character (Utilities|Casting|CastToBP_PlayerCharacter OtherActor)
    (:then
      (Variables|Default|SetObject%20To%20Move _asbp_player_character)
      (CallFunction|FindNearestCheckpoint))
    (:CastFailed
      (bind _asbp_berry_pickup (Utilities|Casting|CastToBP_BerryPickup OtherActor))
      (Variables|Default|SetObject%20To%20Move _asbp_berry_pickup)
      (CallFunction|FindNearestCheckpoint))))

(event Custom|Find%20Nearest%20Checkpoint
  (bind _returnvalue (Actor|GetComponentbyClass "/Script/Engine.PrimitiveComponent"))
  ;[1 1 1] Find nearest checkpoint
  (for _array_element (Variables|Default|GetCheckpoins)
    (if (== (Variables|Default|GetLowest%20Dot%20Product) 0.0)
      (Variables|Default|SetLowest%20Dot%20Product (Math|Vector|DotProduct (Transformation|GetActorLocation (Variables|Default|GetObject%20To%20Move)) (Transformation|GetActorLocation _array_element)))
      (elif (< (Math|Vector|DotProduct (Transformation|GetActorLocation (Variables|Default|GetObject%20To%20Move)) (Transformation|GetActorLocation _array_element)) (Variables|Default|GetLowest%20Dot%20Product))
        (Variables|Default|SetLowest%20Dot%20Product (Math|Vector|DotProduct (Transformation|GetActorLocation (Variables|Default|GetObject%20To%20Move)) (Transformation|GetActorLocation _array_element)))
        (Variables|Default|SetClosest%20Checkpoint _array_element))))
  ;;[1 0.3976 0.3178] Checks if object uses simulate physics, toggles it for stopping movement
  (if (Class|SceneComponent|IsAnySimulatingPhysics _returnvalue)
    (Physics|SetSimulatePhysics _returnvalue false)
    (Physics|SetSimulatePhysics _returnvalue true))
  (Transformation|Teleport (Variables|Default|GetObject%20To%20Move) (Transformation|GetActorLocation (Variables|Default|GetClosest%20Checkpoint)) "0, 0, 0")
  (Variables|Default|SetLowest%20Dot%20Product 0.0))

(event EventBeginPlay
  ;[1 1 1] Get all checkpoints on start
  (bind _outactors (Actor|GetAllActorsOfClass "/Game/GameContent/Blueprints/PlayerSafetyNet/BP_CheckpointTester.BP_CheckpointTester_C"))
  (Variables|Default|SetCheckpoins _outactors))

(fn ConstructionScript)