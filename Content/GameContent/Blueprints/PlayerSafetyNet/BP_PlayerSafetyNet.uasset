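; Player safety net that teleports a BP_PlayerCharacter entering its SafetyCollisionBox to a random navigable location.
; The overlap stores the character and runs FindSuitablePosition, which queries navigable points around it from a default radius.
; Each non-zero result is saved and doubles the radius; a near-zero result ends the loop, and the character moves to the last saved point.
; A debug "Hello" print fires on every iteration.
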(event OnComponentBeginOverlap(SafetyCollisionBox)
  (params (OverlappedComponent :type Primitive%20Component%20Object%20Reference) (OtherActor :type Actor%20Object%20Reference) (OtherComp :type Primitive%20Component%20Object%20Reference) (OtherBodyIndex :type Integer) (bFromSweep :type Boolean) (SweepResult :type Hit%20Result%20Structure%20%28by%20ref%29))
  ;[1 1 1] Detect Player entering net
  (bind _asbp_player_character (Utilities|Casting|CastToBP_PlayerCharacter OtherActor))
  (Variables|Default|SetAs%20BP%20Player%20Character _asbp_player_character)
  (CallFunction|FindSuitablePosition))

(event Custom|Find%20Suitable%20Position
  (bind _as_bp_player_character (Variables|Default|GetAs%20BP%20Player%20Character))
  ;[1 1 1] Find suitable space to teleport player
  (Variables|Default|SetPosFound true)
  (Variables|Default|SetCheckRadius (Variables|Default|GetCheckRadiusDefault))
  (while (Variables|Default|GetPosFound)
    (bind _randomlocation (Class|NavigationSystemV1|GetRandomLocationinNavigableRadius (Transformation|GetActorLocation _as_bp_player_character) (Variables|Default|GetCheckRadius) 0 0))
    (Development|PrintString "Hello")
    (if (Utilities|Operators|EqualEqual :A _randomlocation :ErrorTolerance 0.1)
      (Variables|Default|SetPosFound false)
      (else
        (Variables|Default|SetCheckRadius (* (Variables|Default|GetCheckRadius) 2.0))
        (Variables|Default|SetTeleportPosition _randomlocation))))
  (Transformation|SetActorLocation _as_bp_player_character (Variables|Default|GetTeleportPosition) false false))

(fn ConstructionScript)