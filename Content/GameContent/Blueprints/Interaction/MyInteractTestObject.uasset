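; A test interactable actor that spins its cube when the player interacts with it.
; The Interact event plays a timeline that lerps the cube's current world rotation toward a target rotation.
; A sphere collider's begin and end overlaps cast to BP_PlayerCharacter and turn its interaction UI on and off as the player approaches or leaves.
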(event OnComponentBeginOverlap(SphereCollider)
  (params (OverlappedComponent :type Primitive%20Component%20Object%20Reference) (OtherActor :type Actor%20Object%20Reference) (OtherComp :type Primitive%20Component%20Object%20Reference) (OtherBodyIndex :type Integer) (bFromSweep :type Boolean) (SweepResult :type Hit%20Result%20Structure%20%28by%20ref%29))
  ;[1 1 1] Show/Hide UI when near object
  (bind _asbp_player_character (Utilities|Casting|CastToBP_PlayerCharacter OtherActor))
  (Class|InteractUI|InteractUI _asbp_player_character))

(event OnComponentEndOverlap(SphereCollider)
  (params (OverlappedComponent :type Primitive%20Component%20Object%20Reference) (OtherActor :type Actor%20Object%20Reference) (OtherComp :type Primitive%20Component%20Object%20Reference) (OtherBodyIndex :type Integer))
  ;[1 1 1] Show/Hide UI when near object
  (bind _asbp_player_character (Utilities|Casting|CastToBP_PlayerCharacter OtherActor))
  (Class|InteractUI|InteractUIOff _asbp_player_character))

(event EventInteract
  (bind _cube (Variables|Default|GetCube))
  ;[1 1 1] Spin on interact
  (bind _alpha (Timeline|Timeline Play)
    (:Update
      (Transformation|SetWorldRotation _cube (Math|Rotator|Lerp(Rotator) (Transformation|GetWorldRotation _cube) (Variables|Default|GetTargetRotation) _alpha) false false))))

(fn ConstructionScript)