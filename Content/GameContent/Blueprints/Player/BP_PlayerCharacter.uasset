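; Player character Blueprint that handles inventory pickups, help prompts, animal scanning and pausing.
; Interface events forward pickup, item checks and visibility toggles to BPInventoryComponent, and show or hide a help panel with progress or halt text.
; Scanning messages the Animal through BPI_Scannable, while pause input opens a menu with UI-only input.
; A debug key toggles the HUD camera widget, but the HUD creation chain here is disconnected.
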(event Custom|HideHelpPanel
  ;[0.3953 0.2782 1] PickUp Interface for Inventory Items
  (Widget|RemovefromParent (Variables|Default|GetHelpPanel)))

(event Custom|InventoryHasItem
  (params (ItemName :type String))
  ;[0.3953 0.2782 1] PickUp Interface for Inventory Items
  (Default|InventoryItemCheck (Variables|Default|GetBP_InventoryComponent) ItemName))

(event Custom|Show%20Help%20Panel
  (params (FoundItem :type Boolean))
  (bind _helppanel (Variables|Default|GetHelpPanel))
  ;[0.3953 0.2782 1] PickUp Interface for Inventory Items
  (if FoundItem
    (Default|SetText _helppanel (Variables|Default|GetProgressText))
    (else
      (Default|SetText _helppanel (Variables|Default|GetHaltText))))
  (UserInterface|Viewport|AddtoViewport (Variables|Default|GetHelpPanel) 0))

(event Input|EnhancedActionEvents|EnhancedInputActionIA_Pause
  (params (ActionValue :type Boolean) (ElapsedSeconds :type Float%20%28double-precision%29) (TriggeredSeconds :type Float%20%28double-precision%29) (InputAction :type Input%20Action%20Object%20Reference :default "/Game/GameContent/Blueprints/UI/PauseMenu/IA_Pause.IA_Pause"))
  (bind _returnvalue (Game|GetPlayerController 0))
  (:Started
    (bind _returnvalue_2 (UserInterface|CreateWidget "/Game/GameContent/Blueprints/UI/PauseMenu/W_PauseMenu.W_PauseMenu_C"))
    (UserInterface|Viewport|AddtoViewport _returnvalue_2 0)
    (Variables|/Script/Engine.PlayerController|SetbShowMouseCursor _returnvalue true)
    (Input|SetInputModeUIOnly _returnvalue 0 "DoNotLock" false)
    (Game|SetGamePaused true)))

(event EventBeginPlay
  (bind _returnvalue (UserInterface|CreateWidget "/Game/GameContent/Blueprints/UI/HelpPanel/WB_HelpPanel.WB_HelpPanel_C"))
  (Variables|Default|SetHelpPanel _returnvalue)
  (EventDispatchers|BindEventtoEDonInventoryFilterComplete (Variables|Default|GetBP_InventoryComponent) (EventDispatchers|CreateEvent :!event Custom|Show%20Help%20Panel)))

(event EventActivateAnimal
  ;[1 0.1562 0.1562] Scan interface to scanned animals
  (if (Utilities|DoesObjectImplementInterface (Variables|Default|Get_Animal) "/Game/GameContent/Blueprints/BPInterfaces/BPI_Scannable.BPI_Scannable_C")
    (Class|BPIScannable|OnScanned(Message) (Variables|Default|Get_Animal))))

(event EventPickUpInventoryItem
  (params (interactItem :type Actor%20Object%20Reference))
  ;[1 0.1567 0.1567] PickUp Interface for Inventory Items
  (Default|AddItem (Variables|Default|GetBP_InventoryComponent) interactItem))

(event EventInventoryBPAction
  ;[1 0.1567 0.1567] Inventory Visibility Toggle Interface
  (Default|ToggleInventory (Variables|Default|GetBP_InventoryComponent)))

(event Input|KeyboardEvents|7
  (params (Key :type Key%20Structure :default "None"))
  (bind _playerhud (Variables|Default|GetPlayerHUD))
  ;[1 1 1] Blueprint for Widget Testing (insert begin play into create widget component)
  (:Pressed
    (Default|ToggleCameraWidgeton _playerhud))
  (:Released
    (Default|ToggleCameraWidgetOff _playerhud)))

(fn ConstructionScript)