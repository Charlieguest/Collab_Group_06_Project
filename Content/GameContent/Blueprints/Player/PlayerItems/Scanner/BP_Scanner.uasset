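; Player scanner item that plays the Niagara scan effect when a scan begins.
; On BeginPlay it caches the player character, whose ScanVFXSpawner component supplies the spawn location and rotation.
; BeginScan spawns the effect there unattached, then destroys it after a delay based on its queried play length plus a short margin.
; The Blueprint handles only the visuals, with no detection logic.
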(event EventBeginPlay
  (bind _asbp_player_character (Utilities|Casting|CastToBP_PlayerCharacter (Game|GetPlayerCharacter 0)))
  (Variables|Default|SetAs%20BP%20Player%20Character _asbp_player_character))

(event EventBeginScan
  (bind _as_bp_player_character (Variables|Default|GetAs%20BP%20Player%20Character))
  (bind _scanvfxspawner (Variables|/Game/GameContent/Blueprints/Player/BP_PlayerCharacter.BP_PlayerCharacter_C|GetScanVFXSpawner _as_bp_player_character))
  (bind _returnvalue (Niagara|SpawnSystematLocation "/Game/Art/VFX/NS_Scanner.NS_Scanner" (Transformation|GetWorldLocation _scanvfxspawner) (Transformation|GetWorldRotation _scanvfxspawner)))
  (bind _returnvalue_2 (Animation|GetPlayLength _returnvalue))
  (Utilities|FlowControl|Delay (+ _returnvalue_2 1.0))
  (Components|DestroyComponent _returnvalue))

(fn ConstructionScript)