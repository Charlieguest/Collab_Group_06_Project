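; Player inventory component that stores picked items in six fixed slots and shows them in a toggleable widget panel.
; BeginPlay creates WB_InventoryPanel and sizes the Items array, and ToggleInventory adds or removes the panel from the viewport.
; AddItem copies a BP_InventoryItem's data into the first slot with an empty name, then refreshes the panel through LoadInventory.
; A full inventory silently ignores new items.
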(event Custom|AddItem
  (params (Item :type Actor%20Object%20Reference))
  ;[1 1 1 1 30] Looping through and adding the selected Item to the Inventory if there is space
  (bind _asbp_inventory_item (Utilities|Casting|CastToBP_InventoryItem Item))
  (Variables|Default|SetItemToAdd (Variables|/Script/CollabGroup06Project.InventoryItem|Get_ItemData _asbp_inventory_item))
  (for (_array_element _array_index) (Variables|Default|GetItems)
    (if (not (Variables|Default|GetAddedItem))
      (Variables|Default|SetArray%20Index _array_index)
      (if (Utilities|Enum|Equal(Enum) (._ItemName (Utilities|Struct|BreakItemData _array_element)) "")
        (Utilities|Array|SetArrayElem (Variables|Default|GetItems) (Variables|Default|GetArray%20Index) (Utilities|Struct|MakeItemData (._ItemName (Utilities|Struct|BreakItemData (Variables|Default|GetItemToAdd))) (._Thumbnail (Utilities|Struct|BreakItemData (Variables|Default|GetItemToAdd))) (._Mesh (Utilities|Struct|BreakItemData (Variables|Default|GetItemToAdd)))))
        (Variables|Default|SetAddedItem true)
        (Default|LoadInventory (Variables|Default|GetInventoryPanel) self))))
  (Variables|Default|SetAddedItem false))

(event Custom|Toggle%20Inventory
  (bind _inventorypanel (Variables|Default|GetInventoryPanel))
  ;[0.2299 0.2304 1] Showing and Hiding Inventory
  (if (Widget|IsVisible (Variables|Default|GetInventoryPanel))
    (Widget|RemovefromParent _inventorypanel)
    (else
      (UserInterface|Viewport|AddtoViewport _inventorypanel 0))))

(event EventBeginPlay
  ;[0.5035 1 0.4828] Creating Widget and Setting Empty Item Icons size
  (bind _returnvalue (UserInterface|CreateWidget "/Game/GameContent/Blueprints/UI/Inventory/WB_InventoryPanel.WB_InventoryPanel_C"))
  (Variables|Default|SetInventoryPanel _returnvalue)
  (Utilities|Array|Resize (Variables|Default|GetItems) 6)
  (Default|LoadInventory (Variables|Default|GetInventoryPanel) self))