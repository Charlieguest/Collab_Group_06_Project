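; Teleporter plant actor that sends the player to a linked partner plant when they enter its collision box.
; On overlap it stores the actor, checks it is the player character, waits a delay, then calls OnTeleportedTo on LinkedPlant.
; The receiving plant pulls the stored actor from its own LinkedPlant, so links must be mutual, and moves it to TeleportPoint.
; The receiver's cooldown blocks an immediate bounce back.
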(event OnComponentBeginOverlap(BoxCollision)
  (params (OverlappedComponent :type Primitive%20Component%20Object%20Reference) (OtherActor :type Actor%20Object%20Reference) (OtherComp :type Primitive%20Component%20Object%20Reference) (OtherBodyIndex :type Integer) (bFromSweep :type Boolean) (SweepResult :type Hit%20Result%20Structure%20%28by%20ref%29))
  ;[0.3748 0.3747 1] Plant Entered
  ;;[1 1 1] Player Enters Plant
  (if (not (Variables|Default|GetCoolDownActive))
    (bind _output_get (Variables|Default|SetPlayerCharacter OtherActor))
    (Development|PrintString (Utilities|GetDisplayName _output_get))
    ;;[1 1 1] Check if player
    (Utilities|Casting|CastToBP_PlayerCharacter (Variables|Default|GetPlayerCharacter))
    ;;[1 1 1] Call partnered plant
    (Utilities|FlowControl|Delay (Variables|Default|GetTeleportDelay))
    (CallFunction|OnTeleportedto (Variables|Default|GetLinked%20Plant%20))))

(event Custom|OnTeleportedTo
  (bind _linked_plant_ (Variables|Default|GetLinked%20Plant%20))
  (bind _teleportpoint (Variables|Default|GetTeleportPoint))
  (bind _playercharacter (Variables|BP_TeleportPlant_C|GetPlayerCharacter _linked_plant_))
  ;[0.3065 1 0.3381] Teleported from other plant
  ;;[1 1 1] Move player to teleport point
  (Variables|Default|SetCoolDownActive true)
  (Utilities|IsValid _playercharacter
    (:Is%20Valid
      (Development|PrintString "DEBUG- Teleported Player")
      (Transformation|Teleport _playercharacter (Transformation|GetWorldLocation _teleportpoint) (Transformation|GetWorldRotation _teleportpoint))
      (Utilities|FlowControl|Delay (Variables|Default|GetCoolDownDuration))
      (Variables|Default|SetCoolDownActive false))))

(fn ConstructionScript)